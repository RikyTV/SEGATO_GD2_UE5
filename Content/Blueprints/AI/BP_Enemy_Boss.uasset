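; Boss enemy Blueprint that extends its parent with boss sword-trace points and an on-screen health bar.
; BeginPlay swaps in the boss trace point arrays and hides the inherited Widget component.
; Player overlap with SphereHealthTrigger while alive creates WB_BossHealth and, a tick later, hands its bar to BPCStats.
; Die flags death, ragdolls the mesh, disables movement and capsule collision, and hides the boss bar.
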(event `self.ReceiveBeginPlay`
  (`parent.ReceiveBeginPlay`)
  (set `self.StartSwordTracePosArr` (`self.Boss Attack Start Trace Pos`))
  (set `self.EndSwordTracePosArr` (`self.Boss Attack End Trace Pos`))
  (`SceneComponent.SetVisibility` (`self.Widget`) false false))

(event `self.Sphere Health Trigger.OnComponentBeginOverlap`
  (params (OverlappedComponent :type "PrimitiveComponent Object Reference") (OtherActor :type "Actor Object Reference") (OtherComp :type "PrimitiveComponent Object Reference") (OtherBodyIndex :type Integer) (bFromSweep :type Boolean) (SweepResult :type "HitResult Structure (by ref)"))
  (if (not (`self.IsDead`))
    (cast `/Game/ThirdPerson/Blueprints/BP_ThirdPersonCharacter` OtherActor)
    (bind _returnvalue (`|CreateWidget` "/Game/UI/HUD/WB_BossHealth.WB_BossHealth_C"))
    (bind _output_get (set `self.Boss Health Widget` _returnvalue))
    (`UserWidget.AddToViewport` _output_get 0)
    (`KismetSystemLibrary.DelayUntilNextTick`)
    (`/Game/Blueprints/BPC_Stats.Set Health Progress Bar` (`self.BPC_Stats`) (`/Game/UI/HUD/WB_BossHealth.HealthBar` (`self.Boss Health Widget`)))
    (`SceneComponent.SetVisibility` (`self.Widget`) false false)))

(event `/Game/Blueprints/BPI_Damage.Die`
  (set `self.IsDead` true)
  (`PrimitiveComponent.SetSimulatePhysics` (`self.Mesh`) true)
  (`CharacterMovementComponent.DisableMovement` (`self.CharacterMovement`))
  (bind _output_get (set `self.Boss Health Widget` (stale `self.Sphere Health Trigger.OnComponentBeginOverlap` _returnvalue)))
  (set `Widget.Visibility` "Hidden" _output_get)
  (`PrimitiveComponent.SetCollisionEnabled` (`self.CapsuleComponent`) "NoCollision")
  (`SceneComponent.SetVisibility` (`self.Widget`) false false))

(fn `UserConstructionScript`
  (`parent.UserConstructionScript`))